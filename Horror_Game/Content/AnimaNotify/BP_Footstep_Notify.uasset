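; Animation notify that plays surface-specific footstep sounds when it fires on a valid mesh.
; GetSurface traces down from player character 0, rather than the notifying mesh's owner, and plays wood, brick, dirt, fabric or metal audio at the hit point.
; Other surfaces reach a play-sound call with no sound assigned.
; It also sets a surface number, which Received_Notify checks only to return true.
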(fn `GetSurface`
  (returns (Surface :type "Float (double-precision)"))
  (locals (`Surface Type Num` :type "Float (double-precision)"))
  (bind _returnvalue (`Actor.K2_GetActorLocation` (`GameplayStatics.GetPlayerCharacter` 0)))
  (bind (_outhit _returnvalue_2) (`KismetSystemLibrary.LineTraceSingle` _returnvalue (- _returnvalue (0.0 0.0 150.0)) "TraceTypeQuery1"))
  (if _returnvalue_2
    (switch `EPhysicalSurface` (`GameplayStatics.GetSurfaceType` _outhit)
      (:`SurfaceType_Default`
        (set `local.Surface Type Num` 1.0)
        (bind (_bblockinghit _binitialoverlap _time _distance _location) (`GameplayStatics.BreakHitResult` _outhit))
        (`GameplayStatics.PlaySoundAtLocation` null _location (struct) 1.0 1.0 0.0 null null null null))
      (:`SurfaceType1`
        (set `local.Surface Type Num` 2.0)
        (`GameplayStatics.PlaySoundAtLocation` "/Game/Audio/Wood/WoodFootsteps.WoodFootsteps" _location (struct) 1.0 1.0 0.0 null null null null))
      (:`SurfaceType2`
        (set `local.Surface Type Num` 3.0)
        (`GameplayStatics.PlaySoundAtLocation` "/Game/Audio/Brick/BrickFootsteps.BrickFootsteps" _location (struct) 1.0 1.0 0.0 null null null null))
      (:`SurfaceType3`
        (set `local.Surface Type Num` 4.0)
        (`GameplayStatics.PlaySoundAtLocation` "/Game/Audio/Dirt/DirtFootsteps.DirtFootsteps" _location (struct) 1.0 1.0 0.0 null null null null))
      (:`SurfaceType4`
        (set `local.Surface Type Num` 5.0)
        (`GameplayStatics.PlaySoundAtLocation` "/Game/Audio/Tent/FabricFootsteps.FabricFootsteps" _location (struct) 1.0 1.0 0.0 null null null null))
      (:`SurfaceType5`
        (set `local.Surface Type Num` 6.0)
        (`GameplayStatics.PlaySoundAtLocation` "/Game/Audio/Metal/MetalFootsteps.MetalFootsteps" _location (struct) 1.0 1.0 0.0 null null null null)))
    (return (`local.Surface Type Num`))))

(fn `Received_Notify`
  (params (MeshComp :type "SkeletalMeshComponent Object Reference") (Animation :type "AnimSequenceBase Object Reference") (EventReference :type "AnimNotifyEventReference Structure (by ref)"))
  (returns (ReturnValue :type Boolean))
  (locals (`Surface Type Num` :type "Float (double-precision)"))
  (`/Engine/EditorBlueprintResources/StandardMacros.IsValid` MeshComp
    (:`Is Valid`
      (bind _surface (`self.GetSurface`))
      (bind _output_get (set `local.Surface Type Num` _surface))
      (`|ExecutionSequence`
        (:`then_0`
          (if (== _output_get 2.0)
            (return true)))
        (:`then_1`
          (if (== _output_get 3.0)
            (return true)))
        (:`then_2`
          (if (== _output_get 4.0)
            (return true)))
        (:`then_3`
          (if (== _output_get 5.0)
            (return true)))
        (:`then_4`
          (if (== _output_get 6.0)
            (return true)))))
    (:`Is Not Valid`
      (return true))))