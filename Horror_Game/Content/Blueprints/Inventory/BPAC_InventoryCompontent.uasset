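; Inventory actor component that holds a list of item slots for its owner.
; On BeginPlay it fills the slot array with a configurable number of entries, each carrying its index and a true flag.
; AddItem is a stub that only prints the item ID and amount and returns success, without writing to the slots.
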(event `self.ReceiveBeginPlay`
  (`self.Initialize Slot`))

(fn `Add Item`
  (params (`Item ID` :type String) (Amount :type Integer))
  (returns (`Success?` :type Boolean))
  (`KismetSystemLibrary.PrintString` (`KismetStringLibrary.Concat_StrStr` "Item " `Item ID` "Added to inventory with amount:" (`KismetStringLibrary.Conv_IntToString` Amount)))
  (return true))

(fn `Initialize Slot`
  (for _index (range (`self.Num of Inventory Slots`))
    (`KismetArrayLibrary.Array_Add` (`self.Inventory Slots`) (make `/Game/Blueprints/Inventory/Struct_InventorySlotData` true (struct :`ItemCategory` "NewEnumerator0") _index))))