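; Objective trigger actor that shows an objective title and description on screen when the player first enters its box, which is sized in the construction script.
; It creates the objective widget at BeginPlay, then on overlap fades it in, reverses the fade after a delay and flags the objective as in progress.
; A completion event reuses the widget with a "Completed Objective" title and translucent content text, fading it in and out again.
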(event `self.ReceiveBeginPlay`
  (bind _returnvalue (`|CreateWidget` "/Game/Blueprints/UI/Player/WBP_Objective.WBP_Objective_C" null (`self.Objective Title Text`) (`self.Objective Content Text`)))
  (set `self.WBP_ObejectiveWidgetRef` _returnvalue))

(event `self.Objective Box.OnComponentBeginOverlap`
  (params (OverlappedComponent :type "PrimitiveComponent Object Reference") (OtherActor :type "Actor Object Reference") (OtherComp :type "PrimitiveComponent Object Reference") (OtherBodyIndex :type Integer) (bFromSweep :type Boolean) (SweepResult :type "HitResult Structure (by ref)"))
  (bind _wbp_obejectivewidgetref (`self.WBP_ObejectiveWidgetRef`))
  (bind _wbp_obejectivewidgetref_2 (`self.WBP_ObejectiveWidgetRef`))
  (bind _objectivefade (`/Game/Blueprints/UI/Player/WBP_Objective.ObjectiveFade` _wbp_obejectivewidgetref_2))
  (if (== OtherActor (`GameplayStatics.GetPlayerCharacter` 0))
    (`/Engine/EditorBlueprintResources/StandardMacros.DoOnce` false
      (:`Completed`
        (set `/Game/Blueprints/UI/Player/WBP_Objective.ObjectiveTitleText` (`self.Objective Title Text`) _wbp_obejectivewidgetref)
        (set `/Game/Blueprints/UI/Player/WBP_Objective.ObjectiveContentText` (`self.Objective Content Text`) _wbp_obejectivewidgetref)
        (`TextBlock.SetColorAndOpacity` (`/Game/Blueprints/UI/Player/WBP_Objective.ObjeciveContent` _wbp_obejectivewidgetref) (make `SlateColor` (make `LinearColor` 1.0 1.0 1.0 1.0)))
        (`UserWidget.AddToViewport` _wbp_obejectivewidgetref_2 0)
        (`UserWidget.PlayAnimation` _wbp_obejectivewidgetref_2 _objectivefade 0.0 1 "Forward" 1.0 false)
        (`KismetSystemLibrary.Delay` 5.0)
        (`UserWidget.PlayAnimation` _wbp_obejectivewidgetref_2 _objectivefade 0.0 1 "Reverse" 1.0 false)
        (set `self.ObjectiveInProgress` true)))))

(event `Comlpeted Objective`
  (bind _wbp_obejectivewidgetref (`self.WBP_ObejectiveWidgetRef`))
  (bind _objectivefade (`/Game/Blueprints/UI/Player/WBP_Objective.ObjectiveFade` _wbp_obejectivewidgetref))
  (set `/Game/Blueprints/UI/Player/WBP_Objective.ObjectiveTitleText` "Completed Objective" (`self.WBP_ObejectiveWidgetRef`))
  (`TextBlock.SetColorAndOpacity` (`/Game/Blueprints/UI/Player/WBP_Objective.ObjeciveContent` _wbp_obejectivewidgetref) (make `SlateColor` (make `LinearColor` 1.0 0.0 1.0 0.5)))
  (`UserWidget.PlayAnimation` _wbp_obejectivewidgetref _objectivefade 0.0 1 "Forward" 1.0 false)
  (`KismetSystemLibrary.Delay` 3.0)
  (`UserWidget.PlayAnimation` _wbp_obejectivewidgetref _objectivefade 0.0 1 "Reverse" 1.0 false))

(fn `UserConstructionScript`
  (`BoxComponent.SetBoxExtent` (`self.Objective Box`) (`self.Objective Box Size`) true))