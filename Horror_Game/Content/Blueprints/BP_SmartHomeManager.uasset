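; BP_SmartHomeManager mirrors the player's game state to a real smart light through Home Assistant webhooks.
; Setters for flashlight, chase and death states store their flag, then call UpdateSmartLight.
; That event picks one webhook by priority: death, then AI chase, then flashlight on or off.
; SendWebhook fires it as a JSON POST request through the VaRest plugin, without handling the response.
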(event `SetFlashlightState`
  (params (Flashlight :type Boolean))
  (set `self.FlashlightOn` Flashlight)
  (`self.UpdateSmartLight`))

(event `UpdateSmartLight`
  (if (`self.IsDead`)
    (`self.SendWebhook(WebhookURL)` "http://homeassistant.local:8123/api/webhook/ue5_player_death")
    (elif (`self.IsBeingChased`)
      (`self.SendWebhook(WebhookURL)` "http://homeassistant.local:8123/api/webhook/ue5_ai_chase")
      (elif (`self.FlashlightOn`)
        (`self.SendWebhook(WebhookURL)` "http://homeassistant.local:8123/api/webhook/ue5_flashlight_on")
        (else
          (`self.SendWebhook(WebhookURL)` "http://homeassistant.local:8123/api/webhook/ue5_flashlight_off"))))))

(event `SetChaseState`
  (params (Chase :type Boolean))
  (set `self.IsBeingChased` Chase)
  (`self.UpdateSmartLight`))

(event `SetDeathState`
  (params (Death :type Boolean))
  (set `self.IsDead` Death)
  (`self.UpdateSmartLight`))

(event `SendWebhook(WebhookURL)`
  (params (NewParam :type String))
  (bind _returnvalue (`VaRestSubsystem.ConstructVaRestRequestExt` (subsystem `VaRestSubsystem`) "POST" "json"))
  (`VaRestRequestJSON.SetURL` _returnvalue NewParam)
  (`VaRestRequestJSON.ExecuteProcessRequest` _returnvalue))

(fn `UserConstructionScript`)