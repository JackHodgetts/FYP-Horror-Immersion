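; BP_ItemMaster is a pickup item actor that players collect by walking into it.
; On BeginPlay it looks up its ItemID in DT_InventroyItemData and caches the row as its item data.
; When a BP_ThirdPersonCharacter overlaps its sphere, it adds the item and amount to that character's inventory component.
; On success it shows a HUD pickup notification and destroys itself.
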(event `self.ReceiveBeginPlay`
  (`self.Initialize Item Data Structure`))

(event `self.Sphere.OnComponentBeginOverlap`
  (params (OverlappedComponent :type "PrimitiveComponent Object Reference") (OtherActor :type "Actor Object Reference") (OtherComp :type "PrimitiveComponent Object Reference") (OtherBodyIndex :type Integer) (bFromSweep :type Boolean) (SweepResult :type "HitResult Structure (by ref)"))
  (bind _asbp_third_person_character (cast `/Game/ThirdPerson/Blueprints/BP_ThirdPersonCharacter` OtherActor))
  (bind _success_ (`/Game/Blueprints/Inventory/BPAC_InventoryCompontent.Add Item` (`/Game/ThirdPerson/Blueprints/BP_ThirdPersonCharacter.BPAC_InventoryCompontent` _asbp_third_person_character) (`self.Item ID`) (`self.Amount`)))
  (if _success_
    (`/Game/Blueprints/UI/WBP_PlayerHUD.Add Item Notifcation` (`/Game/ThirdPerson/Blueprints/BP_ThirdPersonCharacter.Player HUD Ref` _asbp_third_person_character) (`self.Item Data Struct`) (`self.Amount`))
    (`self.K2_DestroyActor`)))

(fn `Initialize Item Data Structure`
  (bind _returnvalue (`|GetDataTableRow` "/Game/Blueprints/Items/DT_InventroyItemData.DT_InventroyItemData" (`KismetStringLibrary.Conv_StringToName` (`self.Item ID`)))
    (:`then`
      (set `self.Item Data Struct` _returnvalue))))

(fn `UserConstructionScript`)