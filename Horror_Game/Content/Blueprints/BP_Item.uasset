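; BP_Item is an interactable item actor that shows proximity icons and destroys itself after the player interacts with it.
; Outer and inner overlap spheres, sized in the construction script, toggle far and near interact icons for the player character.
; Tick polls the player's IsInteracting and HitActor, calling Interacted to print and destroy the item after a short delay.
; The Interact function is a stub returning false.
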(event `Interacted`
  (`KismetSystemLibrary.PrintString` "Interacted")
  (`KismetSystemLibrary.Delay` 1.0)
  (`self.K2_DestroyActor`))

(event `self.ReceiveBeginPlay`
  (bind _asbp_third_person_character (cast `/Game/ThirdPerson/Blueprints/BP_ThirdPersonCharacter` (`GameplayStatics.GetPlayerCharacter` 0)))
  (set `self.BP Player Ref` _asbp_third_person_character))

(event `self.ReceiveTick`
  (params (DeltaSeconds :type "Float (single-precision)"))
  (bind _bp_player_ref (`self.BP Player Ref`))
  (if (and (`/Game/ThirdPerson/Blueprints/BP_ThirdPersonCharacter.Is Interacting?` _bp_player_ref) (== (`/Game/ThirdPerson/Blueprints/BP_ThirdPersonCharacter.Hit Actor` _bp_player_ref) self))
    (`self.Interacted`)))

(event `self.innerSphereCollision.OnComponentBeginOverlap`
  (params (OverlappedComponent :type "PrimitiveComponent Object Reference") (OtherActor :type "Actor Object Reference") (OtherComp :type "PrimitiveComponent Object Reference") (OtherBodyIndex :type Integer) (bFromSweep :type Boolean) (SweepResult :type "HitResult Structure (by ref)"))
  (if (== OtherActor (`GameplayStatics.GetPlayerCharacter` 0))
    (`SceneComponent.SetVisibility` (`self.innerInteractIcon`) true false)
    (`SceneComponent.SetVisibility` (`self.outerInteractIcon`) false false)))

(event `self.innerSphereCollision.OnComponentEndOverlap`
  (params (OverlappedComponent :type "PrimitiveComponent Object Reference") (OtherActor :type "Actor Object Reference") (OtherComp :type "PrimitiveComponent Object Reference") (OtherBodyIndex :type Integer))
  (if (== (`GameplayStatics.GetPlayerCharacter` 0) OtherActor)
    (`SceneComponent.SetVisibility` (`self.innerInteractIcon`) false false)
    (`SceneComponent.SetVisibility` (`self.outerInteractIcon`) true false)))

(event `self.outerSphereCollision.OnComponentBeginOverlap`
  (params (OverlappedComponent :type "PrimitiveComponent Object Reference") (OtherActor :type "Actor Object Reference") (OtherComp :type "PrimitiveComponent Object Reference") (OtherBodyIndex :type Integer) (bFromSweep :type Boolean) (SweepResult :type "HitResult Structure (by ref)"))
  (if (== OtherActor (`GameplayStatics.GetPlayerCharacter` 0))
    (`SceneComponent.SetVisibility` (`self.outerInteractIcon`) true false)))

(event `self.outerSphereCollision.OnComponentEndOverlap`
  (params (OverlappedComponent :type "PrimitiveComponent Object Reference") (OtherActor :type "Actor Object Reference") (OtherComp :type "PrimitiveComponent Object Reference") (OtherBodyIndex :type Integer))
  (if (== (`GameplayStatics.GetPlayerCharacter` 0) OtherActor)
    (`SceneComponent.SetVisibility` (`self.outerInteractIcon`) false false)))

(fn `Interact`
  (params (Interacter :type "Character Object Reference"))
  (returns (`Did Interact?` :type Boolean))
  (return false))

(fn `UserConstructionScript`
  (`SphereComponent.SetSphereRadius` (`self.innerSphereCollision`) (`self.InnerSphereRadius`) true)
  (`SphereComponent.SetSphereRadius` (`self.outerSphereCollision`) (`self.OuterSphereRadius`) true))